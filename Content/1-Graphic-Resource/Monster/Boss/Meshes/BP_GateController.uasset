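; Boss-area gate actor that shatters when it takes damage.
; At BeginPlay the fracture mesh is hidden and non-simulating while the static mesh stands in.
; On any damage it swaps to the fracture mesh, enables physics, triggers the FSMaterField actor or component to break it, and plays a random stone-hit sound.
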(event `self.ReceiveBeginPlay`
  (bind _fracturemesh (`self.FractureMesh`))
  (`SceneComponent.SetVisibility` _fracturemesh false false)
  (`PrimitiveComponent.SetSimulatePhysics` _fracturemesh false))

(event `self.ReceiveAnyDamage`
  (params (Damage :type "Float (single-precision)") (DamageType :type "DamageType Object Reference") (InstigatedBy :type "Controller Object Reference") (DamageCauser :type "Actor Object Reference"))
  (bind _fracturemesh (`self.FractureMesh`))
  (`SceneComponent.SetVisibility` _fracturemesh true false)
  (`SceneComponent.SetVisibility` (`self.StaticMesh`) false false)
  (`PrimitiveComponent.SetSimulatePhysics` _fracturemesh true)
  (`/Engine/EditorResources/FieldNodes/FS_MasterField.CE_Trigger` (`self.FS_MaterField`))
  (`GameplayStatics.PlaySound2D` "/Game/Rolling-Kiwi/Sounds/Hit/PlayerAttack/SC_Hit_Player_Stone_Random.SC_Hit_Player_Stone_Random" 1.0 1.0 0.0 null null))

(fn `UserConstructionScript`)