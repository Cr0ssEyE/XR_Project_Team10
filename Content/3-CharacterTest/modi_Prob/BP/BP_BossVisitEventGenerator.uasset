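; Boss arena trigger actor that switches the player's music to the boss BGM on overlap and stages the boss intro.
; If the GameInstance reports the boss as unvisited, it hides the boss and starts the level sequence through SequencePlayer.
; A callback bound at BeginPlay to the sequence's stop reveals the boss, activates its AI, dissolves the blocking crystal, disables Box collision and adds a dummy boss health widget.
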(event `self.ReceiveBeginPlay`
  (add `MovieSceneSequencePlayer.OnStop` (`/Game/3-CharacterTest/modi_Prob/BP/BP_SequencePlayer.Level Sequence Actor` (`self.Sequence Player`)) (delegate `ActivateAI`)))

(event `self.ReceiveActorBeginOverlap`
  (params (OtherActor :type "Actor Object Reference"))
  (bind _askwplayer_character (cast `KWPlayerCharacter` OtherActor))
  (bind _returnvalue (`KWPlayerCharacter.GetMainAudioComponent` _askwplayer_character))
  (`AudioComponent.SetSound` _returnvalue "/Game/Rolling-Kiwi/Sounds/BGM/143_BGM_Boss_Cue.143_BGM_Boss_Cue")
  (`AudioComponent.Play` _returnvalue 0.0)
  (bind _askwgame_instance (cast `KWGameInstance` (`GameplayStatics.GetGameInstance`)))
  (bind _returnvalue_2 (`KWGameInstance.GetBossVisited` _askwgame_instance))
  (if (not _returnvalue_2)
    (`self.SetActorHiddenInGame` (`self.BossMonster`) true)
    (`/Game/3-CharacterTest/modi_Prob/BP/BP_SequencePlayer.SequencePlayEvent` (`self.Sequence Player`))))

(event `ActivateAI`
  (bind _bossmonster (`self.BossMonster`))
  (`self.SetActorHiddenInGame` _bossmonster false)
  (`KWBossMonsterHohonu.ActivateAI` _bossmonster)
  (`/Game/3-CharacterTest/modi_Prob/BP/BP_Trigger_Created_Crystals.Dissolve Event` (`self.Blocking Crystal`))
  (`PrimitiveComponent.SetCollisionEnabled` (`self.Box`) "NoCollision")
  (bind _returnvalue (`|CreateWidget` "/Game/40-Second-Round-Table/WB_DummyBossHealth.WB_DummyBossHealth_C" (`GameplayStatics.GetPlayerController` 0)))
  (`UserWidget.AddToViewport` _returnvalue 0))

(fn `UserConstructionScript`)