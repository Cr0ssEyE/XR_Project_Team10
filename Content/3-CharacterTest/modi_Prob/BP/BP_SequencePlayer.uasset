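; BP_SequencePlayer plays an assigned Level Sequence as an in-game cutscene, taking the player out of view and control while it runs.
; BeginPlay creates the sequence player and binds its finished callback.
; SequencePlayEvent hides the controlled pawn, disables its input, starts playback and toggles all widget visibility through the KWPlayerCharacter's widget controller.
; On finish, the pawn and input are restored and the widgets are toggled again.
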(event `SequencePlayEvent`
  (bind _returnvalue (`GameplayStatics.GetPlayerController` 0))
  (bind _returnvalue_2 (`Controller.K2_GetPawn` _returnvalue))
  (`self.SetActorHiddenInGame` _returnvalue_2 true)
  (`MovieSceneSequencePlayer.Play` (stale `self.ReceiveBeginPlay` _output_get))
  (`self.DisableInput` _returnvalue_2 _returnvalue)
  (bind _askwplayer_character (cast `KWPlayerCharacter` _returnvalue_2))
  (bind _returnvalue_3 (`KWPlayerCharacter.GetWidgetController` _askwplayer_character))
  (`KWPlayerWidgetController.ToggleAllWidgetVisibility` _returnvalue_3))

(event `self.ReceiveBeginPlay`
  (bind (_outactor _returnvalue) (`LevelSequencePlayer.CreateLevelSequencePlayer` (`self.Level Sequence`)))
  (bind _output_get (set `self.Level Sequence Actor` _returnvalue))
  (add `MovieSceneSequencePlayer.OnFinished` _output_get (delegate `SequenceEndEvent`)))

(event `SequenceEndEvent`
  (bind _returnvalue (`GameplayStatics.GetPlayerController` 0))
  (bind _returnvalue_2 (`Controller.K2_GetPawn` _returnvalue))
  (`self.SetActorHiddenInGame` _returnvalue_2 false)
  (`self.EnableInput` _returnvalue_2 _returnvalue)
  (bind _askwplayer_character (cast `KWPlayerCharacter` _returnvalue_2))
  (bind _returnvalue_3 (`KWPlayerCharacter.GetWidgetController` _askwplayer_character))
  (`KWPlayerWidgetController.ToggleAllWidgetVisibility` _returnvalue_3))

(fn `UserConstructionScript`)