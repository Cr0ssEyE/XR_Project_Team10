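; Crystal mesh actor that starts without collision and, judging by its name and logic, materializes through a dissolve effect when triggered.
; BeginPlay creates a dynamic material instance with Dissolve_Main at its low starting value and disables collision.
; DissolveEvent, not called within this Blueprint, plays a Timeline as an update loop that raises the parameter by a fixed, frame-rate-dependent step, enabling collision partway and stopping at the upper limit.
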(event `self.ReceiveBeginPlay`
  (bind _staticmeshcomponent0 (`self.StaticMeshComponent0`))
  (bind _returnvalue (`PrimitiveComponent.CreateDynamicMaterialInstance` _staticmeshcomponent0 0 (`PrimitiveComponent.GetMaterial` _staticmeshcomponent0 0) "None"))
  (bind _output_get (set `self.Material Instance` _returnvalue))
  (`MaterialInstanceDynamic.SetScalarParameterValue` _output_get "Dissolve_Main" -4.0)
  (`PrimitiveComponent.SetCollisionEnabled` _staticmeshcomponent0 "NoCollision"))

(event `self.ReceiveActorBeginOverlap`
  (params (OtherActor :type "Actor Object Reference")))

(event `Dissolve Event`
  (`Timeline|Timeline` :`NewTime` 0.01 :!label _label
    (:`Update`
      (bind _returnvalue (`MaterialInstanceDynamic.K2_GetScalarParameterValue` (`self.Material Instance`) "Dissolve_Main"))
      (if (>= _returnvalue 4.0)
        (goto _label :!via `Stop`)
        (elif (>= _returnvalue 1.0)
          (`PrimitiveComponent.SetCollisionEnabled` (`self.StaticMeshComponent0`) "QueryAndPhysics")
          (bind _returnvalue_2 (+ _returnvalue 0.05))
          (`MaterialInstanceDynamic.SetScalarParameterValue` (`self.Material Instance`) "Dissolve_Main" _returnvalue_2)
          (else
            (`MaterialInstanceDynamic.SetScalarParameterValue` (`self.Material Instance`) "Dissolve_Main" _returnvalue_2)))))))

(fn `UserConstructionScript`)