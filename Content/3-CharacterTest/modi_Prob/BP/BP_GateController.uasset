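; Destructible gate controller that shatters when damaged and dissolves up to two linked crystal walls, CrystalWallA and CrystalWallB.
; On damage it swaps the static mesh for a physics-simulated fracture mesh, triggers the FSMaterField field, plays a stone hit sound and calls DissolveEvent on the walls.
; After a short delay, a timeline steps down the fracture material's Dissolve_Main parameter by a fixed amount per update, then destroys the actor.
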(event `self.ReceiveBeginPlay`
  (bind _fracturemesh (`self.FractureMesh`))
  (`SceneComponent.SetVisibility` _fracturemesh false false)
  (`PrimitiveComponent.SetSimulatePhysics` _fracturemesh false)
  (bind _returnvalue (`PrimitiveComponent.CreateDynamicMaterialInstance` _fracturemesh 0 (`PrimitiveComponent.GetMaterial` _fracturemesh 0) "None"))
  (bind _output_get (set `self.Fracture Material` _returnvalue))
  (`MaterialInstanceDynamic.SetScalarParameterValue` _output_get "Dissolve_Main" 1.0))

(event `self.ReceiveAnyDamage`
  (params (Damage :type "Float (single-precision)") (DamageType :type "DamageType Object Reference") (InstigatedBy :type "Controller Object Reference") (DamageCauser :type "Actor Object Reference"))
  (bind _crystal_wall_a (`self.Crystal Wall A`))
  (bind _crystal_wall_b (`self.Crystal Wall B`))
  (bind _fracturemesh (`self.FractureMesh`))
  (bind _fracture_material (`self.Fracture Material`))
  (`PrimitiveComponent.SetCollisionEnabled` (`self.StaticMesh`) "NoCollision")
  (`SceneComponent.SetVisibility` _fracturemesh true false)
  (`SceneComponent.SetVisibility` (`self.StaticMesh`) false false)
  (`PrimitiveComponent.SetSimulatePhysics` _fracturemesh true)
  (`/Engine/EditorResources/FieldNodes/FS_MasterField.CE_Trigger` (`self.FS_MaterField`))
  (`GameplayStatics.PlaySound2D` "/Game/Rolling-Kiwi/Sounds/Hit/PlayerAttack/SC_Hit_Player_Stone_Random.SC_Hit_Player_Stone_Random" 1.0 1.0 0.0 null null)
  (`|ExecutionSequence`
    (:`then_0`
      (`/Engine/EditorBlueprintResources/StandardMacros.IsValid` _crystal_wall_a
        (:`Is Valid`
          (`/Game/3-CharacterTest/modi_Prob/BP/BP_Trigger_Deleted_Crystals.Dissolve Event` _crystal_wall_a))
        (:`Is Not Valid`
          _))
      (`/Engine/EditorBlueprintResources/StandardMacros.IsValid` _crystal_wall_b
        (:`Is Valid`
          (`/Game/3-CharacterTest/modi_Prob/BP/BP_Trigger_Deleted_Crystals.Dissolve Event` _crystal_wall_b))))
    (:`then_1`
      (`KismetSystemLibrary.Delay` 1.0)
      (`Timeline|Timeline` :`NewTime` 0.01
        (:`Update`
          (bind _returnvalue (`MaterialInstanceDynamic.K2_GetScalarParameterValue` _fracture_material "Dissolve_Main"))
          (if (<= _returnvalue 0.0)
            (`self.K2_DestroyActor`)
            (else
              (`MaterialInstanceDynamic.SetScalarParameterValue` _fracture_material "Dissolve_Main" (+ _returnvalue -0.005)))))))))

(fn `UserConstructionScript`)