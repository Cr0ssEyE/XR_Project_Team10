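; A crystal mesh actor that dissolves away and destroys itself when its DissolveEvent is called.
; BeginPlay creates a dynamic material instance on the static mesh.
; DissolveEvent plays a timeline whose updates lower the Dissolve_Main parameter by a fixed step each tick, destroying the actor and stopping the timeline once it reaches zero.
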(event `self.ReceiveBeginPlay`
  (bind _staticmeshcomponent0 (`self.StaticMeshComponent0`))
  (bind _returnvalue (`PrimitiveComponent.CreateDynamicMaterialInstance` _staticmeshcomponent0 0 (`PrimitiveComponent.GetMaterial` _staticmeshcomponent0 0) "None"))
  (set `self.Material Instance` _returnvalue))

(event `Dissolve Event`
  (bind _material_instance (`self.Material Instance`))
  (`Timeline|Timeline` :`NewTime` 0.01 :!label _label
    (:`Update`
      (bind _returnvalue (`MaterialInstanceDynamic.K2_GetScalarParameterValue` _material_instance "Dissolve_Main"))
      (if (<= _returnvalue 0.0)
        (`self.K2_DestroyActor`)
        (goto _label :!via `Stop`)
        (else
          (`MaterialInstanceDynamic.SetScalarParameterValue` _material_instance "Dissolve_Main" (+ _returnvalue -0.02)))))))

(fn `UserConstructionScript`)