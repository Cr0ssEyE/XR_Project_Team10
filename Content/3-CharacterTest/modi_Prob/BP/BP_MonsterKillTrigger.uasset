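; BP_MonsterKillTrigger is a trigger that dissolves a target object once all of its assigned monsters are destroyed.
; On BeginPlay it counts up to three valid monster references, binds to each one's OnDestroyed event and hides its Sphere component.
; Each destruction increments a stack, and reaching the count calls DissolveEvent on TargetObject.
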(event `self.ReceiveBeginPlay`
  (bind _triggermonstera (`self.TriggerMonsterA`))
  (bind _triggermonsterb (`self.TriggerMonsterB`))
  (bind _triggermonsterc (`self.TriggerMonsterC`))
  (bind _returnvalue (+ (`self.MaxTrigger`) 1))
  (`/Engine/EditorBlueprintResources/StandardMacros.IsValid` _triggermonstera
    (:`Is Valid`
      (set `self.MaxTrigger` _returnvalue)
      (add `self.OnDestroyed` _triggermonstera (delegate `OnDestroyed_Event`)))
    (:`Is Not Valid`
      _))
  (`/Engine/EditorBlueprintResources/StandardMacros.IsValid` _triggermonsterb
    (:`Is Valid`
      (set `self.MaxTrigger` _returnvalue)
      (add `self.OnDestroyed` _triggermonsterb (delegate `OnDestroyed_Event`)))
    (:`Is Not Valid`
      _))
  (`/Engine/EditorBlueprintResources/StandardMacros.IsValid` _triggermonsterc
    (:`Is Valid`
      (set `self.MaxTrigger` _returnvalue)
      (add `self.OnDestroyed` _triggermonsterc (delegate `OnDestroyed_Event`)))
    (:`Is Not Valid`
      _))
  (`SceneComponent.SetVisibility` (`self.Sphere`) false false))

(event `OnDestroyed_Event` :!signature `self.OnDestroyed`
  (params (DestroyedActor :type "Actor Object Reference"))
  (bind _output_get (set `self.TriggerStack` (+ 1 (`self.TriggerStack`))))
  (if (>= _output_get (`self.MaxTrigger`))
    (`/Game/3-CharacterTest/modi_Prob/BP/BP_Trigger_Deleted_Crystals.Dissolve Event` (`self.Target Object`))))

(fn `UserConstructionScript`)